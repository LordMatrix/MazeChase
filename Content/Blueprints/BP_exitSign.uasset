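; BP_exitSign is the maze chase exit: the player character overlapping its Box wins the game.
; On that overlap, if the gamemode's GameWon flag is unset, it clears all widgets and shows WBP_GameWon with the sign's whole-second lifetime as the time.
; It then tells BP_MazeChaseGamemode to fade to the menu and sets GameWon, so later overlaps do nothing.
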(event OnComponentBeginOverlap(Box)
  (params (OverlappedComponent :type Primitive%20Component%20Object%20Reference) (OtherActor :type Actor%20Object%20Reference) (OtherComp :type Primitive%20Component%20Object%20Reference) (OtherBodyIndex :type Integer) (bFromSweep :type Boolean) (SweepResult :type Hit%20Result%20Structure%20%28by%20ref%29))
  (bind _asbp_maze_chase_gamemode (Utilities|Casting|CastToBP_MazeChaseGamemode (Game|GetGameMode)))
  (if (not (Variables|/Game/Blueprints/BP_MazeChaseGamemode.BP_MazeChaseGamemode_C|Getgame_won _asbp_maze_chase_gamemode))
    (Utilities|Casting|CastToMazeChaseCharacter OtherActor)
    (Viewport|RemoveAllWidgets)
    (bind _returnvalue (UserInterface|CreateWidget "/Game/Blueprints/WBP_GameWon.WBP_GameWon_C"))
    (UserInterface|Viewport|AddtoViewport _returnvalue 0)
    (Default|SetTime _returnvalue (Math|Float|Truncate (Actor|GetGameTimeSinceCreation)))
    (Default|FadetoMenu _asbp_maze_chase_gamemode)
    (Variables|/Game/Blueprints/BP_MazeChaseGamemode.BP_MazeChaseGamemode_C|Setgame_won _asbp_maze_chase_gamemode true)))

(fn ConstructionScript)