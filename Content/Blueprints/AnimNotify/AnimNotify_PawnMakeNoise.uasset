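; Animation notify that makes a MazeChaseCharacter emit a noise when the notify fires in an animation.
; It casts the mesh owner to MazeChaseCharacter and calls MakeNoise on its noise emitter at the actor's location.
; Loudness comes from the notify's own volume, or from a scaled-down copy of the character's step loudness when that volume is zero or less.
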(fn ReceivedNotify
  (params (MeshComp :type Skeletal%20Mesh%20Component%20Object%20Reference) (Animation :type Anim%20Sequence%20Base%20Object%20Reference))
  (bind _volume_in (Variables|Default|Getvolume_in))
  (bind _asmaze_chase_character (Utilities|Casting|CastToMazeChaseCharacter (Components|GetOwner MeshComp)))
  (if (<= _volume_in 0.0)
    (LocalVariables|Setvolume_out (* (Variables|/Script/MazeChase.MazeChaseCharacter|Getstep_loudness_ _asmaze_chase_character) 0.1))
    (else
      (LocalVariables|Setvolume_out _volume_in)))
  (Class|PawnNoiseEmitterComponent|MakeNoise (Variables|/Script/MazeChase.MazeChaseCharacter|Getnoise_emiter_ _asmaze_chase_character) _asmaze_chase_character (LocalVariables|Getvolume_out) (Transformation|GetActorLocation _asmaze_chase_character))
  (return true))