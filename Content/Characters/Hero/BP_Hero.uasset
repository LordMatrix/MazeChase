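; BP_Hero is the player character Blueprint, with sneak and run movement and death on contact with a Minotaur.
; Sneak and Run inputs switch walk speed, with Run ignored while PawnSneaking is set.
; Capsule overlap and hit events share one Minotaur cast that sets PawnDead and prints a death message.
; An unconnected leftover graph would briefly hide a door and disable its collision, or switch to flying, but never runs.
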(event OnComponentBeginOverlap(CapsuleComponent)
  (params (OverlappedComponent :type Primitive%20Component%20Object%20Reference) (OtherActor :type Actor%20Object%20Reference) (OtherComp :type Primitive%20Component%20Object%20Reference) (OtherBodyIndex :type Integer) (bFromSweep :type Boolean) (SweepResult :type Hit%20Result%20Structure%20%28by%20ref%29))
  (Utilities|Casting|CastToMinotaur (stale OnComponentHit(CapsuleComponent) OtherActor))
  (Variables|Default|Setpawn_dead_ true)
  (Development|PrintString "YOU ARE DEAD"))

(event OnComponentHit(CapsuleComponent)
  (params (HitComponent :type Primitive%20Component%20Object%20Reference) (OtherActor :type Actor%20Object%20Reference) (OtherComp :type Primitive%20Component%20Object%20Reference) (NormalImpulse :type Vector :default "0, 0, 0") (Hit :type Hit%20Result%20Structure%20%28by%20ref%29))
  (Utilities|Casting|CastToMinotaur OtherActor)
  (Variables|Default|Setpawn_dead_ true)
  (Development|PrintString "YOU ARE DEAD"))

(event Input|ActionEvents|InputActionFly
  (params (Key :type Key%20Structure :default "AnyKey")))

(event Input|ActionEvents|InputActionRun
  (params (Key :type Key%20Structure :default "AnyKey"))
  (bind _charactermovement (Variables|Character|GetCharacterMovement))
  (:Pressed
    (if (not (Variables|Default|Getpawn_sneaking_))
      (Variables|/Script/Engine.CharacterMovementComponent|SetMaxWalkSpeed _charactermovement 9e+02)))
  (:Released
    (if (not (Variables|Default|Getpawn_sneaking_))
      (Variables|/Script/Engine.CharacterMovementComponent|SetMaxWalkSpeed _charactermovement 6e+02))))

(event Input|ActionEvents|InputActionSneak
  (params (Key :type Key%20Structure :default "AnyKey"))
  (bind _charactermovement (Variables|Character|GetCharacterMovement))
  (:Pressed
    (Variables|/Script/Engine.CharacterMovementComponent|SetMaxWalkSpeed _charactermovement 3e+02)
    (Variables|Default|Setpawn_sneaking_ true))
  (:Released
    (Variables|/Script/Engine.CharacterMovementComponent|SetMaxWalkSpeed _charactermovement 6e+02)
    (Variables|Default|Setpawn_sneaking_ false)))

(fn ConstructionScript)